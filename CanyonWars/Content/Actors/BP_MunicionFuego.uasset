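; BP_MunicionFuego is a fire ammunition actor that is collected by shooting or otherwise damaging it.
; Any damage swaps three spheres to a yellow-red material, clears the material override on a fourth, and subtracts from its Vida health.
; At zero health it prints that the ammo was obtained and destroys itself; no ammo is granted here, only debug messages.
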(event Game|Damage|EventAnyDamage
  (params (Damage :type Float%20%28single-precision%29) (DamageType :type Damage%20Type%20Object%20Reference) (InstigatedBy :type Controller%20Object%20Reference) (DamageCauser :type Actor%20Object%20Reference))
  (Development|PrintString "Municion de fuego alcanzada")
  (Rendering|Material|SetMaterial (Variables|Default|GetSphere1) 0 "/Game/Materials/AmarilloRojizo.AmarilloRojizo")
  (Rendering|Material|SetMaterial (Variables|Default|GetSphere) 0 "/Game/Materials/AmarilloRojizo.AmarilloRojizo")
  (Rendering|Material|SetMaterial (Variables|Default|GetSphere2) 0 "/Game/Materials/AmarilloRojizo.AmarilloRojizo")
  (Rendering|Material|SetMaterial (Variables|Default|GetSphere3) 0 0)
  (bind _output_get (Variables|Default|SetVida (- (Variables|Default|GetVida) Damage)))
  (if (<= _output_get 0.0)
    (Development|PrintString "Munición de fuego obtenida")
    (Actor|DestroyActor)))

(fn ConstructionScript)